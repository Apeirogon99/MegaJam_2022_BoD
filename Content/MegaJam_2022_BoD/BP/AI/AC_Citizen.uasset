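; AI controller for citizen pawns that keeps them wandering between point objects in the level and can set their skeletal mesh.
; A sphere trace ahead of the pawn, widening after each miss, picks the next point using BP_GM_Battle's random stream.
; AIMoveTo heads to a reachable spot nearby, searching again on success or after a delay on failure.
; C2S/S2C events drive this loop, leaving an older MoveToPoint/NextPoint loop unused.
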(event `self.ReceiveBeginPlay`
  (`self.C2S_FindPointObject` (`self.K2_GetPawn`)))

(event `SpawnMove`
  (`self.C2S_FindPointObject` (`self.K2_GetPawn`)))

(event `self.ReceiveTick`
  (params (DeltaSeconds :type "Float (single-precision)")))

(event `MoveToPoint`
  (params (Point :type "Vector Structure"))
  (`|AIMoveTo` null Point null 100.0
    (:`OnSuccess`
      _)
    (:`OnFail`
      (`KismetSystemLibrary.Delay` 2.0)))
  (`self.NextPoint`))

(event `NextPoint`
  (bind _returnvalue (`self.K2_GetPawn`))
  (bind _returnvalue_2 (+ (`self.K2_GetActorLocation` _returnvalue) (* (`self.GetActorForwardVector` _returnvalue) 700.0)))
  (bind (_outhits _returnvalue_3) (`KismetSystemLibrary.SphereTraceMultiForObjects` _returnvalue_2 (+ _returnvalue_2 (1.0 0.0 0.0)) (`self.Radius`) (`|MakeArray` "ObjectTypeQuery7" :!type "EObjectTypeQuery Enum") false (`|MakeArray` (`self.CrruentPoint`)) "ForDuration" :!label _label))
  (if _returnvalue_3
    (bind (_bblockinghit _binitialoverlap _time _distance _location _impactpoint _normal _impactnormal _physmat _hitactor) (`GameplayStatics.BreakHitResult` (`|GetArrayItem` _outhits (`KismetMathLibrary.RandomInteger` (`KismetArrayLibrary.Array_Length` _outhits)))))
    (set `self.CrruentPoint` _hitactor)
    (set `self.Radius` 500.0)
    (`self.MoveToPoint` (`NavigationSystemV1.K2_GetRandomReachablePointInRadius` _impactpoint 100.0 null null))
    (else
      (set `self.Radius` (+ (`self.Radius`) 500.0))
      (`KismetSystemLibrary.Delay` 2.0)
      (goto _label))))

(event `C2S_SuccessToMove`
  (params (Pawn :type "Pawn Object Reference"))
  (`self.C2S_FindPointObject` Pawn))

(event `C2S_FailToMove`
  (params (Pawn :type "Pawn Object Reference"))
  (`KismetSystemLibrary.K2_SetTimerDelegate` (delegate `TryAgain`) 2.0))

(event `C2S_FindPointObject`
  (params (ControllerPawn :type "Pawn Object Reference"))
  (bind _returnvalue (+ (`self.K2_GetActorLocation` ControllerPawn) (* (`self.GetActorForwardVector` ControllerPawn) (`self.ForwardDistance`))))
  (`/Engine/EditorBlueprintResources/StandardMacros.IsValid` ControllerPawn
    (:`Is Valid`
      (bind _asbp_gm_battle (cast `/Game/MegaJam_2022_BoD/Online/Battle/BP_GM_Battle` (`GameplayStatics.GetGameMode`))
        (:`then`
          (`/Game/MegaJam_2022_BoD/Online/Battle/BP_GM_Battle.GetRandomSeed` _asbp_gm_battle)
          (bind (_outhits _returnvalue_2) (`KismetSystemLibrary.SphereTraceMultiForObjects` _returnvalue (+ _returnvalue (1.0 0.0 0.0)) (`self.Radius`) (`|MakeArray` "ObjectTypeQuery7" :!type "EObjectTypeQuery Enum") false (`|MakeArray` (`self.CrruentPoint`)) "ForDuration" :!label _label_2))
          (if _returnvalue_2
            (bind (_bblockinghit _binitialoverlap _time _distance _location _impactpoint _normal _impactnormal _physmat _hitactor) (`GameplayStatics.BreakHitResult` (`|GetArrayItem` _outhits (`KismetMathLibrary.RandomIntegerFromStream` (`KismetArrayLibrary.Array_Length` _outhits) (`/Game/MegaJam_2022_BoD/Online/Battle/BP_GM_Battle.Stream` _asbp_gm_battle)))))
            (set `self.CrruentPoint` _hitactor)
            (set `self.Radius` 600.0)
            (`self.S2C_MoveToPoint` (`NavigationSystemV1.K2_GetRandomReachablePointInRadius` _impactpoint 100.0 null null) ControllerPawn)
            (else
              (set `self.Radius` (+ (`self.Radius`) 600.0))
              (`KismetSystemLibrary.Delay` 2.0)
              (goto _label_2))))
        (:`CastFailed`
          (`KismetSystemLibrary.PrintString` "Failed "))))))

(event `TryAgain`
  (`self.C2S_FindPointObject` (stale `C2S_FailToMove` Pawn)))

(event `S2C_MoveToPoint`
  (params (Point :type "Vector Structure") (Pawn :type "Pawn Object Reference"))
  (`|AIMoveTo` null Point null (`self.Acceptance Radius`)
    (:`OnSuccess`
      (`self.C2S_SuccessToMove` Pawn))
    (:`OnFail`
      (`self.C2S_FailToMove` Pawn))))

(event `SetPlayerMesh`
  (params (NewParam :type "SkeletalMesh Object Reference"))
  (`self.SetPlayerMesh On Server` NewParam (`self.K2_GetPawn`)))

(event `SetPlayerMesh On Server`
  (params (NewMesh :type "SkeletalMesh Object Reference") (NewParam :type "Pawn Object Reference"))
  (bind _asap_citizen (cast `/Game/MegaJam_2022_BoD/BP/AI/AP_Citizen` NewParam))
  (`/Engine/EditorBlueprintResources/ActorMacros.Switch Has Authority`
    (:`Authority`
      (`|ExecutionSequence`
        (:`then_0`
          (`self.SetPlayerMesh On Clinet` (`Character.Mesh` _asap_citizen) NewMesh))
        (:`then_1`
          (`SkinnedMeshComponent.SetSkinnedAssetAndUpdate` (stale `SetPlayerMesh On Clinet` Target) (stale `SetPlayerMesh On Clinet` NewMesh) false :!label _label_3))))))

(event `SetPlayerMesh On Clinet`
  (params (Target :type "SkinnedMeshComponent Object Reference") (NewMesh :type "SkeletalMesh Object Reference"))
  (`/Engine/EditorBlueprintResources/ActorMacros.Switch Has Authority`
    (:`Remote`
      (goto _label_3))))

(fn `OnRep_CrruentPoint`)

(fn `UserConstructionScript`)