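; BP_Clue is a battle-map clue actor that a player destroys by pressing Interact nearby.
; Its Box overlap enables input for the entering FirstPersonCharacter's BPC_Battle controller and disables it on exit.
; The overlap handlers loop over the game mode's cached controller list, but the input toggle follows either way.
; Interact chains DestroyActorServer into DestroyActorClient, named as a server-to-client relay, to destroy the actor.
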(event `self.ReceiveBeginPlay`
  (bind _asbp_gm_battle (cast `/Game/MegaJam_2022_BoD/Online/Battle/BP_GM_Battle` (`GameplayStatics.GetGameMode`)))
  (set `self.Player Controller` (`/Game/MegaJam_2022_BoD/Online/Battle/BP_GM_Battle.PlayerController` _asbp_gm_battle)))

(event `self.Box.OnComponentBeginOverlap`
  (params (OverlappedComponent :type "PrimitiveComponent Object Reference") (OtherActor :type "Actor Object Reference") (OtherComp :type "PrimitiveComponent Object Reference") (OtherBodyIndex :type Integer) (bFromSweep :type Boolean) (SweepResult :type "HitResult Structure (by ref)"))
  (bind _asfirst_person_character (cast `/Game/MegaJam_2022_BoD/Online/Battle/FirstPersonCharacter` OtherActor))
  (bind _asbpc_battle (cast `/Game/MegaJam_2022_BoD/Online/Battle/BPC_Battle` (`Pawn.GetController` _asfirst_person_character)))
  (for _array_element (`self.Player Controller`)
    (if (== _array_element _asbpc_battle)
      (break)))
  (`self.EnableInput` _asbpc_battle))

(event `self.Box.OnComponentEndOverlap`
  (params (OverlappedComponent :type "PrimitiveComponent Object Reference") (OtherActor :type "Actor Object Reference") (OtherComp :type "PrimitiveComponent Object Reference") (OtherBodyIndex :type Integer))
  (bind _asfirst_person_character (cast `/Game/MegaJam_2022_BoD/Online/Battle/FirstPersonCharacter` OtherActor))
  (bind _asbpc_battle (cast `/Game/MegaJam_2022_BoD/Online/Battle/BPC_Battle` (`Pawn.GetController` _asfirst_person_character)))
  (for _array_element (`self.Player Controller`)
    (if (== _array_element _asbpc_battle)
      (break)))
  (`self.DisableInput` _asbpc_battle))

(event `InputAction|Interact`
  (params (Key :type "Key Structure"))
  (:`Pressed`
    (`self.Destroy Actor Server`)
    (`KismetSystemLibrary.PrintString` "Destroy")))

(event `Destroy Actor Server`
  (`self.Destroy Actor Client`))

(event `Destroy Actor Client`
  (`self.K2_DestroyActor`))

(fn `UserConstructionScript`)