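; BP_Teleport is a battle-map teleporter that moves the FirstPersonCharacter between entrance and exit actors sharing a TeleportIndex.
; Overlapping TeleportArea searches all BP_Teleport actors for the opposite end and moves the player to its ExitReference, also applying rotation when returning to an entrance.
; The construction script positions TeleportArea and ExitReference from variables.
; The AbleToSee overlap only casts, with no further effect.
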(event `self.Teleport Area.OnComponentBeginOverlap`
  (params (OverlappedComponent :type "PrimitiveComponent Object Reference") (OtherActor :type "Actor Object Reference") (OtherComp :type "PrimitiveComponent Object Reference") (OtherBodyIndex :type Integer) (bFromSweep :type Boolean) (SweepResult :type "HitResult Structure (by ref)"))
  (bind _asfirst_person_character (cast `/Game/MegaJam_2022_BoD/Online/Battle/FirstPersonCharacter` OtherActor))
  (if (`self.Entrance`)
    (bind _outactors (`GameplayStatics.GetAllActorsOfClass` "BP_Teleport_C"))
    (for _array_element _outactors
      (if (and (== (`/Game/MegaJam_2022_BoD/BP/BattleMap/System/BP_Teleport.Teleport Index` _array_element) (`self.Teleport Index`)) (not (`/Game/MegaJam_2022_BoD/BP/BattleMap/System/BP_Teleport.Entrance` _array_element)))
        (break)))
    (`self.K2_SetActorLocation` _asfirst_person_character (`SceneComponent.K2_GetComponentLocation` (`/Game/MegaJam_2022_BoD/BP/BattleMap/System/BP_Teleport.Exit Reference` _array_element)) false false)
    (else
      (bind _outactors_2 (`GameplayStatics.GetAllActorsOfClass` "BP_Teleport_C"))
      (for _array_element_2 _outactors_2
        (if (and (== (`/Game/MegaJam_2022_BoD/BP/BattleMap/System/BP_Teleport.Teleport Index` _array_element_2) (`self.Teleport Index`)) (and (not (`self.Entrance`)) (`/Game/MegaJam_2022_BoD/BP/BattleMap/System/BP_Teleport.Entrance` _array_element_2)))
          (break)))
      (bind _exit_reference (`/Game/MegaJam_2022_BoD/BP/BattleMap/System/BP_Teleport.Exit Reference` _array_element_2))
      (`self.K2_SetActorLocationAndRotation` _asfirst_person_character (`SceneComponent.K2_GetComponentLocation` _exit_reference) (`SceneComponent.K2_GetComponentRotation` _exit_reference) false false))))

(event `self.Able to See.OnComponentBeginOverlap`
  (params (OverlappedComponent :type "PrimitiveComponent Object Reference") (OtherActor :type "Actor Object Reference") (OtherComp :type "PrimitiveComponent Object Reference") (OtherBodyIndex :type Integer) (bFromSweep :type Boolean) (SweepResult :type "HitResult Structure (by ref)"))
  (cast `/Game/MegaJam_2022_BoD/Online/Battle/FirstPersonCharacter` OtherActor))

(fn `UserConstructionScript`
  (`SceneComponent.K2_SetRelativeTransform` (`self.Teleport Area`) (`self.Transform Teleport`) false false)
  (`SceneComponent.K2_SetRelativeLocation` (`self.Exit Reference`) (`self.Location Exit`) false false))