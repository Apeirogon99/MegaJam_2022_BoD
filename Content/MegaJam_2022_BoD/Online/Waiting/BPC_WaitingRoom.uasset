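; Player controller for the online waiting room, linking lobby UI to ready-state logic.
; S2C_UpdatePlayerLists rebuilds the main widget's list from each player state's nickname and ready flag, and S2C_ShowCountWidget displays the start countdown.
; C2S_UpdatePlayerList writes the ready flag to the player state, runs the game state's all-ready check and notifies the game mode.
; Enter opens the chat box; widget show/hide logic is left unwired.
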(event `self.ReceiveBeginPlay`)

(event `ShowMainWidget`)

(event `Key|Tab`
  (params (Key :type "Key Structure")))

(event `Key|Enter`
  (params (Key :type "Key Structure"))
  (:`Pressed`
    (`W_WaitingMain.OpenChattingBox` (`self.m_WaitingMain`))))

(event `S2C_UpdatePlayerLists`
  (bind _asbw_waiting_main (cast `/Game/MegaJam_2022_BoD/Widget/Watiting/BW_WaitingMain` (`self.m_WaitingMain`)))
  (`/Game/MegaJam_2022_BoD/Widget/Watiting/BW_WaitingMain.ClearList` _asbw_waiting_main)
  (bind _asbgs_waiting_room (cast `/Game/MegaJam_2022_BoD/Online/Waiting/BGS_WaitingRoom` (`GameplayStatics.GetGameState`)))
  (for _array_element (`GameStateBase.PlayerArray` _asbgs_waiting_room)
    (bind _asbps_waiting_room (cast `/Game/MegaJam_2022_BoD/Online/Waiting/BPS_WaitingRoom` _array_element))
    (`/Game/MegaJam_2022_BoD/Widget/Watiting/BW_WaitingMain.UpdatePlayerList` _asbw_waiting_main (`/Game/MegaJam_2022_BoD/Online/Waiting/BPS_WaitingRoom.Ready` _asbps_waiting_room) (`/Game/MegaJam_2022_BoD/Online/Waiting/BPS_WaitingRoom.NickName` _asbps_waiting_room))))

(event `C2S_UpdatePlayerList`
  (params (Ready :type Boolean))
  (bind _asbps_waiting_room (cast `/Game/MegaJam_2022_BoD/Online/Waiting/BPS_WaitingRoom` (`self.PlayerState`)))
  (`/Game/MegaJam_2022_BoD/Online/Waiting/BPS_WaitingRoom.UpdateReady` _asbps_waiting_room Ready)
  (bind _asbgs_waiting_room (cast `/Game/MegaJam_2022_BoD/Online/Waiting/BGS_WaitingRoom` (`GameplayStatics.GetGameState`)))
  (`/Game/MegaJam_2022_BoD/Online/Waiting/BGS_WaitingRoom.IsAllReady` _asbgs_waiting_room)
  (bind _asbgm_waiting_room (cast `/Game/MegaJam_2022_BoD/Online/Waiting/BGM_WaitingRoom` (`GameplayStatics.GetGameMode`)))
  (`/Game/MegaJam_2022_BoD/Online/Waiting/BGM_WaitingRoom.ChangePlayerReady` _asbgm_waiting_room))

(event `S2C_ShowCountWidget`
  (bind _returnvalue (`|CreateWidget` "/Game/MegaJam_2022_BoD/Widget/Watiting/B_StartCount.B_StartCount_C"))
  (`UserWidget.AddToViewport` _returnvalue 0))

(fn `UserConstructionScript`)