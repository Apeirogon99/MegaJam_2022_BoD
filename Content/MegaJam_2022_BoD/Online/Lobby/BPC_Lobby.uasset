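; BPC_Lobby is the lobby Blueprint that puts the main lobby UI on screen and keeps its nickname display updated.
; On BeginPlay it creates the BW_LobbyMain widget if none is valid, adds it to the viewport, then calls GetNickName on its nested BNickName element.
; An UpdateNickName event re-runs that same nickname fetch on demand.
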(event `self.ReceiveBeginPlay`
  (`self.ShowLobbyMain`)
  (`self.GetNickName`))

(event `GetNickName`
  (`W_LobbyNickName.GetNickName` (`/Game/MegaJam_2022_BoD/Widget/Lobby/BW_LobbyMain.B_NickName` (`self.LobbyMain`))))

(event `ShowLobbyMain`
  (`/Engine/EditorBlueprintResources/StandardMacros.IsValid` (`self.LobbyMain`)
    (:`Is Valid`
      _)
    (:`Is Not Valid`
      (bind _returnvalue (`|CreateWidget` "/Game/MegaJam_2022_BoD/Widget/Lobby/BW_LobbyMain.BW_LobbyMain_C"))
      (set `self.LobbyMain` _returnvalue)))
  (`UserWidget.AddToViewport` (`self.LobbyMain`) 0))

(event `self.UpdateNickName`
  (`self.GetNickName`))

(fn `UserConstructionScript`)