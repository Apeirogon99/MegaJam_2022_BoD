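; Battle game mode that assigns Thief or Police jobs to connected players, spawns their characters and populates the match with NPCs.
; BeginPlay seeds a random stream, then splits the NPC budget across all AI_Spawner actors, passing each a freshly seeded stream.
; Once the expected player count connects, jobs are drawn from a depleting pool and characters are possessed at role-specific spawns.
; StartGame then removes players' widgets if NPC spawning is done, otherwise sets a one-second timer.
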(event `self.ReceiveBeginPlay`
  (`self.SetStreamSeed`)
  (`KismetSystemLibrary.PrintString` "Open GM_Battle")
  (`self.SpawnNPC`))

(event `SpawnNPC`
  (if (`self.isStream`)
    (bind _outactors (`GameplayStatics.GetAllActorsOfClass` "/Game/MegaJam_2022_BoD/BP/BattleMap/AI/AI_Spawner.AI_Spawner_C"))
    (bind _output_get (set `self.Spawners` _outactors))
    (if (!= (`KismetArrayLibrary.Array_Length` _output_get) 0)
      (for _array_element _output_get
        (bind _stream (`self.GetRandomSeed`))
        (`/Game/MegaJam_2022_BoD/BP/BattleMap/AI/AI_Spawner.SpawnPlayers` _array_element (/ (`self.MAX_NPC`) (`KismetArrayLibrary.Array_Length` (`self.Spawners`))) _stream))
      (`KismetSystemLibrary.PrintString` "Completed Spawn NPC")
      (set `self.isSpawnNPC` true))
    (else
      (`KismetSystemLibrary.K2_SetTimerDelegate` (`|CreateDelegate` :!event `SpawnNPC`) 1.0))))

(event `SetStreamSeed`
  (`KismetMathLibrary.SeedRandomStream` (`self.Stream`))
  (set `self.isStream` true)
  (`KismetSystemLibrary.PrintString` "Completed random stream seed"))

(event `StartGame`
  (if (`self.isSpawnNPC`)
    (for _array_element (`self.PlayerController`)
      (`/Game/MegaJam_2022_BoD/Online/Battle/BPC_Battle.RemoveWidget` _array_element))
    (else
      (`KismetSystemLibrary.K2_SetTimerDelegate` (`|CreateDelegate` :!event `StartGame`) 1.0))))

(event `SpawnPlayers`
  ;[1 1 1] Spawn & Create Players
  (for _array_element (`self.PlayerController`)
    (bind _asbpc_battle (cast `/Game/MegaJam_2022_BoD/Online/Battle/BPC_Battle` _array_element))
    (bind _asbps_battle (cast `/Game/MegaJam_2022_BoD/Online/Battle/BPS_Battle` (`Controller.PlayerState` _asbpc_battle)))
    (`self.CreatePlayer` (`/Game/MegaJam_2022_BoD/Online/Battle/BPS_Battle.Job` _asbps_battle) _asbpc_battle))
  (`self.StartGame`))

(event `CreatePlayer`
  (params (Job :type "/Game/MegaJam_2022_BoD/Online/Battle/EJob Enum" :default "NewEnumerator2") (Controller :type "/Game/MegaJam_2022_BoD/Online/Battle/BPC_Battle Object Reference"))
  (bind _returnvalue (`Controller.K2_GetPawn` Controller))
  ;[1 1 1] Spawn & Create Players
  (`/Engine/EditorBlueprintResources/StandardMacros.IsValid` _returnvalue
    (:`Is Valid`
      (`Controller.UnPossess` Controller)
      (`self.K2_DestroyActor` _returnvalue))
    (:`Is Not Valid`
      _))
  (switch `/Game/MegaJam_2022_BoD/Online/Battle/EJob` Job
    (:`NewEnumerator2`
      (`KismetSystemLibrary.PrintString` "FAILD Create Player"))
    (:`NewEnumerator0`
      (bind _returnvalue_2 (`|SpawnActorFromClass` "/Game/MegaJam_2022_BoD/Online/Battle/FirstPersonCharacter.FirstPersonCharacter_C" (`self.ThiefSpawn`) "Undefined" "OverrideRootScale" null null))
      (`/Engine/EditorBlueprintResources/StandardMacros.IsValid` _returnvalue_2
        (:`Is Valid`
          (`Controller.Possess` Controller _returnvalue_2)
          (`KismetSystemLibrary.PrintString` "Spawn Thief"))))
    (:`NewEnumerator1`
      (bind _returnvalue_3 (`|SpawnActorFromClass` "/Game/MegaJam_2022_BoD/Online/Battle/FirstPersonCharacter.FirstPersonCharacter_C" (`self.PoliceSpawn`) "Undefined" "OverrideRootScale" null null))
      (`/Engine/EditorBlueprintResources/StandardMacros.IsValid` _returnvalue_3
        (:`Is Valid`
          (`Controller.Possess` Controller _returnvalue_3)
          (`KismetSystemLibrary.PrintString` "Spawn Police"))))))

(event `self.OnConnected`
  (params (controller :type "PC_Battle Object Reference"))
  ;[1 1 1] OnConnected
  (`KismetSystemLibrary.PrintString` (`KismetStringLibrary.Concat_StrStr` "Connected Player : " (`KismetSystemLibrary.GetDisplayName` controller)))
  (bind _asbpc_battle (cast `/Game/MegaJam_2022_BoD/Online/Battle/BPC_Battle` controller))
  (`KismetArrayLibrary.Array_AddUnique` (`self.PlayerController`) _asbpc_battle)
  (bind _asbp_bo_dgame_instance (cast `/Game/MegaJam_2022_BoD/Online/BP_BoDGameInstance` (`GameplayStatics.GetGameInstance`)))
  (if (== (`/Game/MegaJam_2022_BoD/Online/BP_BoDGameInstance.S_PlayerNum` _asbp_bo_dgame_instance) (`KismetArrayLibrary.Array_Length` (`self.PlayerController`)))
    (`self.SetPlayerJob`)))

(event `SetPlayerJob`
  (bind (_outitem _outindex) (`KismetArrayLibrary.Array_RandomFromStream` (`self.Jobs`) (`self.Stream`)))
  ;[1 1 1] SetJob
  (for _array_element (`self.PlayerController`)
    (bind _asbps_battle (cast `/Game/MegaJam_2022_BoD/Online/Battle/BPS_Battle` (`Controller.PlayerState` _array_element)))
    (switch `/Game/MegaJam_2022_BoD/Online/Battle/EJob` _outitem
      (:`NewEnumerator2`
        (`KismetSystemLibrary.PrintString` "FAILD to Setting Job"))
      (:`NewEnumerator0`
        (`/Game/MegaJam_2022_BoD/Online/Battle/BPS_Battle.SetJob` _asbps_battle (`|GetArrayItem` (`self.Jobs`) _outindex) :!label _label)
        (`KismetArrayLibrary.Array_Remove` (`self.Jobs`) _outindex))
      (:`NewEnumerator1`
        (goto _label))))
  (`self.SpawnPlayers`))

(fn `GetRandomSeed`
  (returns (Stream :type "RandomStream Structure"))
  (`KismetMathLibrary.SeedRandomStream` (`self.Stream`))
  (return (`self.Stream`)))

(fn `UserConstructionScript`)